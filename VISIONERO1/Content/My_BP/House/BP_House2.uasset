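; BP_House2 is a house actor that carries a widget component showing a house health UI.
; Both the construction script and BeginPlay cast the HealthWidget's user widget to WBP_HouseHealth and set its House reference to this actor, so the widget can read this house's state.
; It has no other logic; the overlap and tick events are disabled.
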(event `self.ReceiveBeginPlay`
  (bind _aswbp_house_health (cast `/Game/My_BP/Widgets/WBP_HouseHealth` (`WidgetComponent.GetWidget` (`self.HealthWidget`))))
  (set `/Game/My_BP/Widgets/WBP_HouseHealth.House` self _aswbp_house_health))

(fn `UserConstructionScript`
  (bind _aswbp_house_health (cast `/Game/My_BP/Widgets/WBP_HouseHealth` (`WidgetComponent.GetWidget` (`self.HealthWidget`))))
  (set `/Game/My_BP/Widgets/WBP_HouseHealth.House` self _aswbp_house_health))