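; BP_PlayerPawn is the player's pawn, handling HUD creation, unit move orders and the pause menu.
; On BeginPlay it adds the WBP_Wave widget to the viewport.
; SetUnitLocation traces under the cursor on the Visibility channel and sends the Unit to the hit location with AIMoveTo.
; The Pause input uses a FlipFlop to alternately show WBP_Pause and pause the game, or remove it and unpause.
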(event `self.ReceiveBeginPlay`
  (bind _returnvalue (`|CreateWidget` "/Game/My_BP/Widgets/WBP_Wave.WBP_Wave_C" (`GameplayStatics.GetPlayerController` 0)))
  (bind _output_get (set `self.WBP_Wave` _returnvalue))
  (`UserWidget.AddToViewport` _output_get 0))

(event `self.SetUnitLocation`
  (bind _unit (`self.Unit`))
  (bind (_hitresult _returnvalue) (`PlayerController.GetHitResultUnderCursorByChannel` (`GameplayStatics.GetPlayerController` 0) "TraceTypeQuery1" true))
  (if _returnvalue
    (`|AIMoveTo` _unit _unit (`.Location` (`GameplayStatics.BreakHitResult` _hitresult)) null 5.0 true)))

(event `InputAction|Pause` :paused true
  (params (Key :type "Key Structure"))
  (:`Pressed`
    (`/Engine/EditorBlueprintResources/StandardMacros.FlipFlop`
      (:`A`
        (bind _returnvalue (`|CreateWidget` "/Game/My_BP/Widgets/WBP_Pause.WBP_Pause_C" (`GameplayStatics.GetPlayerController` 0)))
        (bind _output_get (set `self.WBP_Pause` _returnvalue))
        (`UserWidget.AddToViewport` _output_get 0)
        (`GameplayStatics.SetGamePaused` true))
      (:`B`
        (`Widget.RemoveFromParent` (`self.WBP_Pause`))
        (`GameplayStatics.SetGamePaused` false)))))

(fn `UserConstructionScript`)