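; BP_EnemyUnit is an enemy unit that hunts and attacks friendly units with a zombie attack montage.
; On BeginPlay it binds itself to its health widget, starts its AI_Enemy behavior tree and sets a looping retarget timer.
; MoveTOGoalActor picks a random BP_FriendUnit inside its detection sphere, moves to it, plays the montage, calls Attack, then repeats after a delay.
; The sphere's begin and end overlap handlers are empty, with their older logic left disconnected.
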(event `self.ReceiveBeginPlay`
  (`|ExecutionSequence`
    (:`then_0`
      (bind _aswbp_unit_health (cast `/Game/My_BP/Widgets/WBP_UnitHealth` (`WidgetComponent.GetWidget` (`self.HealthWidget`))))
      (bind _output_get (set `self.As WBP Unit Health` _aswbp_unit_health))
      (set `/Game/My_BP/Widgets/WBP_UnitHealth.Unit` self _output_get)
      (bind _asai_enemy (cast `/Game/My_BP/Unit/EnemyUnit/AI_Enemy` (`AIBlueprintHelperLibrary.GetAIController` self)))
      (bind _output_get_2 (set `self.As AI Enemy` _asai_enemy))
      (`/Game/My_BP/Unit/EnemyUnit/AI_Enemy.RunBT` _output_get_2))
    (:`then_1`
      (`KismetSystemLibrary.K2_SetTimerDelegate` (delegate `CustomEvent_0`) 3.0 true))))

(event `CustomEvent_0`
  (`self.MoveTOGoalActor`))

(event `self.SphereCollison.OnComponentBeginOverlap`
  (params (OverlappedComponent :type "PrimitiveComponent Object Reference") (OtherActor :type "Actor Object Reference") (OtherComp :type "PrimitiveComponent Object Reference") (OtherBodyIndex :type Integer) (bFromSweep :type Boolean) (SweepResult :type "HitResult Structure (by ref)")))

(event `MoveTOGoalActor`
  (bind _overlappingactors (`PrimitiveComponent.GetOverlappingActors` (`self.SphereCollison`) "/Game/My_BP/Unit/FriendUnit/BP_FriendUnit.BP_FriendUnit_C"))
  (if (> (`KismetArrayLibrary.Array_Length` _overlappingactors) 0)
    (set `self.GoalActor` (`KismetArrayLibrary.Array_Random` _overlappingactors))
    (bind _goalactor (`self.GoalActor`)
      (:`then`
        (`|AIMoveTo` self (`self.K2_GetActorLocation` _goalactor) _goalactor
          (:`OnSuccess`
            (`/Engine/EditorBlueprintResources/StandardMacros.IsValid` _goalactor
              (:`Is Valid`
                (`|PlayMontage` (`self.Mesh`) "/Game/BSP_ZombieAnims/Animations/Standing/Attack/AS_NAAT_Zombie_Attack_LH_Stand_Montage.AS_NAAT_Zombie_Attack_LH_Stand_Montage"
                  (:`OnCompleted`
                    (`self.Attack`)
                    (`KismetSystemLibrary.Delay` 1.0)
                    (`self.GoalActor`
                      (:`then`
                        _)
                      (:`else`
                        (set `self.GoalActor` (`KismetArrayLibrary.Array_Random` (`PrimitiveComponent.GetOverlappingActors` (`self.SphereCollison`) "/Game/My_BP/Unit/FriendUnit/BP_FriendUnit.BP_FriendUnit_C")))))
                    (`self.MoveTOGoalActor`))))))))
      (:`else`))))

(event `self.SphereCollison.OnComponentEndOverlap`
  (params (OverlappedComponent :type "PrimitiveComponent Object Reference") (OtherActor :type "Actor Object Reference") (OtherComp :type "PrimitiveComponent Object Reference") (OtherBodyIndex :type Integer)))

(fn `UserConstructionScript`)