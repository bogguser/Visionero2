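; BP_FriendUnit is a friendly unit that automatically seeks and attacks BP_EnemyUnit actors, with a health widget bound to it on BeginPlay.
; MoveTOGoalActor moves to the current GoalActor via AIMoveTo, or picks a random enemy overlapping SphereCollison when none is valid.
; It attacks on arrival and on some move failures, then calls itself after a delay.
; A looping timer also re-triggers this routine.
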(event `self.ReceiveBeginPlay`
  (bind _aswbp_unit_health (cast `/Game/My_BP/Widgets/WBP_UnitHealth` (`WidgetComponent.GetWidget` (`self.HealthWidget`))))
  (bind _output_get (set `self.As WBP Health` _aswbp_unit_health))
  (set `/Game/My_BP/Widgets/WBP_UnitHealth.Unit` self _output_get)
  (`KismetSystemLibrary.K2_SetTimerDelegate` (delegate `CustomEvent_0`) 2.0 true))

(event `CustomEvent_0`
  (`self.MoveTOGoalActor`))

(event `self.SphereCollison.OnComponentBeginOverlap`
  (params (OverlappedComponent :type "PrimitiveComponent Object Reference") (OtherActor :type "Actor Object Reference") (OtherComp :type "PrimitiveComponent Object Reference") (OtherBodyIndex :type Integer) (bFromSweep :type Boolean) (SweepResult :type "HitResult Structure (by ref)")))

(event `self.SphereCollison.OnComponentEndOverlap`
  (params (OverlappedComponent :type "PrimitiveComponent Object Reference") (OtherActor :type "Actor Object Reference") (OtherComp :type "PrimitiveComponent Object Reference") (OtherBodyIndex :type Integer)))

(event `MoveTOGoalActor`
  (bind _goalactor (`self.GoalActor`)
    (:`then`
      (`|AIMoveTo` self (`self.K2_GetActorLocation` _goalactor) _goalactor
        (:`OnSuccess`
          _)
        (:`OnFail`
          _))
      (`/Engine/EditorBlueprintResources/StandardMacros.IsValid` _goalactor
        (:`Is Valid`
          (`self.Attack`)
          (`KismetSystemLibrary.Delay` 1.0)
          (`self.MoveTOGoalActor`))))
    (:`else`
      (`KismetSystemLibrary.Delay` 0.3)
      (bind _output_get (set `self.GoalActor` (`KismetArrayLibrary.Array_Random` (`PrimitiveComponent.GetOverlappingActors` (`self.SphereCollison`) "/Game/My_BP/Unit/EnemyUnit/BP_EnemyUnit.BP_EnemyUnit_C"))))
      (`/Engine/EditorBlueprintResources/StandardMacros.IsValid` _output_get
        (:`Is Valid`
          (bind _movementresult (`|AIMoveTo` self (`self.K2_GetActorLocation` _output_get) _output_get)
            (:`OnSuccess`
              (`self.Attack` :!label _label)
              (`KismetSystemLibrary.Delay` 1.0)
              (`self.MoveTOGoalActor`))
            (:`OnFail`
              (if (`|EnumEquality` _movementresult "Blocked")
                (goto _label)))))))))

(fn `UserConstructionScript`)