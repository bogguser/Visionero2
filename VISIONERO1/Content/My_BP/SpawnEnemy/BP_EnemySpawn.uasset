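; BP_EnemySpawn is an actor that travels to an end point, spawns a group of enemies, then retreats and removes itself.
; On BeginPlay a timeline drives VInterpTo movement toward EndPoint, acting as a timer rather than supplying the position.
; When it finishes, a loop based on EnemyCount spawns BP_EnemyUnit AI pawns at SpawnPoint.
; A second timeline then eases the actor toward FirstLocation and destroys it on completion.
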(event `self.ReceiveBeginPlay`
  (bind (_returnvalue_location _returnvalue_rotation) (`KismetMathLibrary.BreakTransform` (`self.GetTransform` (`self.SpawnPoint`))))
  (`Timeline|Timeline` :!via `PlayFromStart`
    (:`Update`
      (`self.K2_SetActorLocation` (`KismetMathLibrary.VInterpTo` (`self.K2_GetActorLocation`) (`SceneComponent.K2_GetComponentLocation` (`Actor.RootComponent` (`self.EndPoint`))) (`GameplayStatics.GetWorldDeltaSeconds`) 0.3)))
    (:`Finished`
      (for _ (range (+ (`self.EnemyCount`) 1))
        (`AIBlueprintHelperLibrary.SpawnAIFromClass` "/Game/My_BP/Unit/EnemyUnit/BP_EnemyUnit.BP_EnemyUnit_C" null _returnvalue_location _returnvalue_rotation false null))
      (`Timeline|Timeline_0` :!via `PlayFromStart`
        (:`Update`
          (`self.K2_SetActorLocation` (`KismetMathLibrary.VInterpTo` (`self.K2_GetActorLocation`) (`self.FirstLocation`) (`GameplayStatics.GetWorldDeltaSeconds`) 0.3)))
        (:`Finished`
          (`self.K2_DestroyActor`))))))

(fn `UserConstructionScript`)